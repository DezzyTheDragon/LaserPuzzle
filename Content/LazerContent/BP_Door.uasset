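; BP_Door is a power-driven door that opens once enough power sources are enabled.
; OnPowerEnable and OnPowerDisable adjust PowerCount and compare it against PowerRequired.
; Reaching the threshold plays a timeline that lerps the Arrow component from its relative origin to MoveLocation.
; Dropping below it snaps Arrow back to the origin through a DoOnce that the enable path resets.
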(event `/Game/LazerContent/BPI_Trigger.OnPowerEnable`
  (`/Engine/EditorBlueprintResources/StandardMacros.IncrementInt` (`self.PowerCount`)
    (:`  `
      (if (>= (`self.PowerCount`) (`self.PowerRequired`))
        (`|ExecutionSequence`
          (:`then_0`
            (bind (_direction _alpha) (`Timeline|Timeline` :!via `PlayFromStart`)
              (:`Update`
                (`SceneComponent.K2_SetRelativeLocation` (`self.Arrow`) (`KismetMathLibrary.VLerp` (0.0 0.0 0.0) (`self.MoveLocation`) _alpha) false false))))
          (:`then_1`
            (goto _label :!via `Reset`)))))))

(event `/Game/LazerContent/BPI_Trigger.OnPowerDisable`
  (if (> (`self.PowerCount`) 0)
    (`/Engine/EditorBlueprintResources/StandardMacros.DecrementInt` (`self.PowerCount`)
      (:`  `
        (if (not (>= (`self.PowerCount`) (`self.PowerRequired`)))
          (`/Engine/EditorBlueprintResources/StandardMacros.DoOnce` (not (`self.DoorIsOpen`)) :!label _label
            (:`Completed`
              (`SceneComponent.K2_SetRelativeLocation` (`self.Arrow`) (0.0 0.0 0.0) false false))))))))

(fn `UserConstructionScript`)