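; BP_Filter is a colored laser filter that passes on only the color channels a hitting laser shares exactly with its own Color.
; Construction and BeginPlay tint the plane through a dynamic M_Filter material.
; On a hit, ValidateColor zeroes mismatched RGB channels; if any stays positive, a filtered BP_Laser spawns at the hit point, attached to its source.
; The Lasers map tracks spawned beams by source so OnLaserHitStop can destroy them.
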(event `self.ReceiveBeginPlay`
  (bind _returnvalue (`PrimitiveComponent.CreateDynamicMaterialInstance` (`self.Plane`) 0 "/Game/Materials/M_Filter.M_Filter" "None"))
  (`MaterialInstanceDynamic.SetVectorParameterValue` _returnvalue "Color" (`self.Color`)))

(event `/Game/LazerContent/BPI_Laser.OnLaserHit`
  (params (LaserColor :type "LinearColor Structure") (LaserHitPos :type "Vector Structure") (LaserHitNormal :type "Vector Structure") (LaserStart :type "Vector Structure") (LaserSrc :type "/Game/LazerContent/BP_Laser Object Reference"))
  (bind (_outputcolor _colorvalid) (`self.ValidateColor` LaserColor (`self.Color`)))
  (if _colorvalid
    (bind _returnvalue (`|SpawnActorFromClass` "/Game/LazerContent/BP_Laser.BP_Laser_C" (`KismetMathLibrary.MakeTransform` LaserHitPos (`self.K2_GetActorRotation` LaserSrc)) "Undefined" "MultiplyWithRoot" null _outputcolor true null))
    (`BlueprintMapLibrary.Map_Add` (`self.Lasers`) LaserSrc _returnvalue)
    (`self.K2_AttachToActor` _returnvalue LaserSrc "None" "KeepWorld" "KeepWorld" "KeepRelative" true)))

(event `/Game/LazerContent/BPI_Laser.OnLaserHitStop`
  (params (LaserID :type "/Game/LazerContent/BP_Laser Object Reference") (LaserColor :type "LinearColor Structure"))
  (bind (_value _returnvalue) (`BlueprintMapLibrary.Map_Find` (`self.Lasers`) LaserID))
  (if _returnvalue
    (`self.K2_DestroyActor` _value)))

(fn `UserConstructionScript`
  (bind _returnvalue (`PrimitiveComponent.CreateDynamicMaterialInstance` (`self.Plane`) 0 "/Game/Materials/M_Filter.M_Filter" "None"))
  (`MaterialInstanceDynamic.SetVectorParameterValue` _returnvalue "Color" (`self.Color`)))

(fn `ValidateColor`
  (params (GivenColor :type "LinearColor Structure") (FilterColor :type "LinearColor Structure"))
  (returns (OutputColor :type "LinearColor Structure") (ColorValid :type Boolean))
  (bind _returnvalue (`KismetMathLibrary.SelectFloat` GivenColor_G 0.0 (== GivenColor_G FilterColor_G)))
  (bind _returnvalue_2 (`KismetMathLibrary.SelectFloat` GivenColor_R 0.0 (== GivenColor_R FilterColor_R)))
  (bind _returnvalue_3 (`KismetMathLibrary.SelectFloat` FilterColor_B 0.0 (== GivenColor_B FilterColor_B)))
  (return (make `LinearColor` _returnvalue_2 _returnvalue _returnvalue_3 GivenColor_A) (or (> _returnvalue_2 0.0) (> _returnvalue 0.0) (> _returnvalue_3 0.0))))