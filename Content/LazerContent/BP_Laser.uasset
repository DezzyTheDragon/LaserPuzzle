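; BP_Laser is a colored laser beam actor that fires along its up vector and notifies the actor it hits.
; Each tick a line trace stretches the mesh to the hit or to maximum range, sending hit and stop messages only when the target changes, plus a stop on destruction.
; With SnapToSurface on, a backward trace moves the beam's origin onto a BP_Filter surface behind it.
; A dynamic material instance applies LaserColor at BeginPlay.
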(event `self.ReceiveBeginPlay`
  (`self.ChangeColor`))

(event `self.ReceiveTick`
  (params (DeltaSeconds :type "Float (single-precision)"))
  (`self.SetEndPoint`)
  (if (`self.SnapToSurface`)
    (`self.FindStartPoint`)))

(event `self.ReceiveDestroyed`
  (message `/Game/LazerContent/BPI_Laser.OnLaserHitStop` (`self.LastHitActor`) self (`self.LaserColor`)))

(fn `ChangeColor`
  (bind _returnvalue (`PrimitiveComponent.CreateDynamicMaterialInstance` (`self.StaticMesh`) 0 "/Game/Materials/M_Laser.M_Laser" "None"))
  (`MaterialInstanceDynamic.SetVectorParameterValue` _returnvalue "Color" (`self.LaserColor`)))

(fn `FindStartPoint`
  (bind _returnvalue (* (`self.GetActorUpVector`) 2.0))
  (bind _returnvalue_2 (+ (`self.K2_GetActorLocation`) _returnvalue))
  (bind _outhit (`KismetSystemLibrary.LineTraceSingle` _returnvalue_2 (+ _returnvalue_2 (* (* _returnvalue -1.0) 10.0)) "TraceTypeQuery1"))
  (bind (_bblockinghit _binitialoverlap _time _distance _location _impactpoint _normal _impactnormal _physmat _hitactor) (`GameplayStatics.BreakHitResult` _outhit))
  (if (and _bblockinghit (`KismetMathLibrary.ClassIsChildOf` (`GameplayStatics.GetObjectClass` _hitactor) "/Game/LazerContent/BP_Filter.BP_Filter_C"))
    (`self.K2_SetActorLocation` _impactpoint)))

(fn `InvalidateHitActor`
  (set `self.LastHitActor` null))

(fn `LockTranslation`
  (params (Normal :type "Vector Structure")))

(fn `SetEndPoint`
  (bind _returnvalue (`self.GetActorUpVector`))
  (bind _lasthitactor (`self.LastHitActor`))
  (bind _returnvalue_2 (+ (`self.K2_GetActorLocation`) (* _returnvalue 2.0)))
  (bind _outhit (`KismetSystemLibrary.LineTraceSingle` _returnvalue_2 (+ _returnvalue_2 (* _returnvalue (`self.LaserRange`))) "TraceTypeQuery2"))
  (bind (_bblockinghit _binitialoverlap _time _distance _location _impactpoint _normal _impactnormal _physmat _hitactor _hitcomponent _hitbonename _bonename _hititem _elementindex _faceindex _tracestart) (`GameplayStatics.BreakHitResult` _outhit))
  (`SceneComponent.SetWorldScale3D` (`self.StaticMesh`) (`KismetMathLibrary.MakeVector` 0.05 0.05 (`KismetMathLibrary.SelectFloat` (/ (+ _distance 1.0) 100.0) (/ (`self.LaserRange`) 100.0) _bblockinghit)))
  (if (not (== (`self.LastHitActor`) _hitactor))
    (if (`KismetSystemLibrary.IsValid` _lasthitactor)
      (message `/Game/LazerContent/BPI_Laser.OnLaserHitStop` _lasthitactor self (`self.LaserColor`)))
    (bind _output_get (set `self.LastHitActor` _hitactor))
    (message `/Game/LazerContent/BPI_Laser.OnLaserHit` _output_get (`self.LaserColor`) _impactpoint _impactnormal _tracestart self)))

(fn `UserConstructionScript`)