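; BP_LaserEmitter is a colored laser emitter that spawns a BP_Laser while active.
; The construction script and BeginPlay tint a dynamic emitter material with LaserColor, and BeginPlay starts the laser if IsEmmitting is set.
; OnPowerEnable toggles that state, switching the glow intensity and either spawning a laser at the Arrow, passing it the color, or destroying the current one.
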(event `self.ReceiveBeginPlay`
  (bind _lasercolor (`self.LaserColor`))
  (bind _returnvalue (`PrimitiveComponent.CreateDynamicMaterialInstance` (`self.LaserEmitter`) 2 "/Game/Materials/M_Emitter.M_Emitter" "None"))
  (bind _output_get (set `self.Emmission` _returnvalue))
  (`MaterialInstanceDynamic.SetVectorParameterValue` _output_get "Color" _lasercolor)
  (if (`self.IsEmmitting`)
    (`MaterialInstanceDynamic.SetScalarParameterValue` _output_get "Intensity" 100.0)
    (bind _returnvalue_2 (`|SpawnActorFromClass` "/Game/LazerContent/BP_Laser.BP_Laser_C" (`KismetMathLibrary.MakeTransform` (`SceneComponent.K2_GetComponentLocation` (`self.Arrow`)) (`self.K2_GetActorRotation`)) "Undefined" "MultiplyWithRoot" null _lasercolor null :!label _label))
    (set `self.Laser` _returnvalue_2)))

(event `/Game/LazerContent/BPI_Trigger.OnPowerEnable`
  (bind _emmission (`self.Emmission`))
  (bind _output_get (set `self.IsEmmitting` (not (`self.IsEmmitting`))))
  (if _output_get
    (`MaterialInstanceDynamic.SetScalarParameterValue` _emmission "Intensity" 100.0)
    (goto _label)
    (else
      (`MaterialInstanceDynamic.SetScalarParameterValue` _emmission "Intensity" 0.0)
      (`self.K2_DestroyActor` (`self.Laser`)))))

(fn `UserConstructionScript`
  (bind _returnvalue (`PrimitiveComponent.CreateDynamicMaterialInstance` (`self.LaserEmitter`) 2 "/Game/Materials/M_Emitter.M_Emitter" "None"))
  (`MaterialInstanceDynamic.SetVectorParameterValue` _returnvalue "Color" (`self.LaserColor`)))