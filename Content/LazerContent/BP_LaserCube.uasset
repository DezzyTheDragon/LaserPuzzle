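; Laser relay cube that emits a same-colored beam while a laser hits it.
; OnLaserHit, if idle, stores the source and spawns a BP_Laser at the Arrow, pitched straight down, then attaches it to itself.
; A dynamic emitter material glows in the beam's color once attachment succeeds.
; OnLaserHitStop responds only to the stored source, destroying the beam and darkening the emitter.
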(event `self.ReceiveBeginPlay`
  (`parent.ReceiveBeginPlay`)
  (bind _returnvalue (`PrimitiveComponent.CreateDynamicMaterialInstance` (`self.StaticMesh`) 0 "/Game/Materials/M_Emitter.M_Emitter" " None"))
  (bind _output_get (set `self.EmitterMaterial` _returnvalue))
  (`MaterialInstanceDynamic.SetVectorParameterValue` :`self` _output_get :`ParameterName` "Color"))

(event `/Game/LazerContent/BPI_Laser.OnLaserHit`
  (params (LaserColor :type "LinearColor Structure") (LaserHitPos :type "Vector Structure") (LaserHitNormal :type "Vector Structure") (LaserStart :type "Vector Structure") (LaserSrc :type "/Game/LazerContent/BP_Laser Object Reference"))
  (bind (_returnvalue_roll _returnvalue_pitch _returnvalue_yaw) (`KismetMathLibrary.BreakRotator` (`self.K2_GetActorRotation`)))
  (bind _emittermaterial (`self.EmitterMaterial`))
  (if (not (`self.CurrentlyEmitting`))
    (set `self.LaserSource` LaserSrc)
    (bind _returnvalue (`|SpawnActorFromClass` "/Game/LazerContent/BP_Laser.BP_Laser_C" (`KismetMathLibrary.MakeTransform` (`SceneComponent.K2_GetComponentLocation` (`self.Arrow`)) (`KismetMathLibrary.MakeRotator` _returnvalue_roll -90.0 _returnvalue_yaw)) "Undefined" "MultiplyWithRoot" null LaserColor null))
    (bind _output_get (set `self.Laser` _returnvalue))
    (bind _returnvalue_2 (`self.K2_AttachToActor` _output_get self "LaserPoint" "KeepWorld" "KeepWorld" "KeepRelative" true))
    (if _returnvalue_2
      (set `self.CurrentlyEmitting` true)
      (`MaterialInstanceDynamic.SetScalarParameterValue` _emittermaterial "Intensity" 100.0)
      (`MaterialInstanceDynamic.SetVectorParameterValue` _emittermaterial "Color" LaserColor)
      (else
        (`KismetSystemLibrary.PrintString` "Failed to attach")))))

(event `/Game/LazerContent/BPI_Laser.OnLaserHitStop`
  (params (LaserID :type "/Game/LazerContent/BP_Laser Object Reference") (LaserColor :type "LinearColor Structure"))
  (bind _emittermaterial (`self.EmitterMaterial`))
  (if (== LaserID (`self.LaserSource`))
    (`self.K2_DestroyActor` (`self.Laser`))
    (set `self.CurrentlyEmitting` false)
    (`MaterialInstanceDynamic.SetScalarParameterValue` _emittermaterial "Intensity" 0.0)
    (`MaterialInstanceDynamic.SetVectorParameterValue` :`self` _emittermaterial :`ParameterName` "Color")))

(fn `UserConstructionScript`
  (`parent.UserConstructionScript`))