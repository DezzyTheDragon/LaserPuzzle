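; BP_Mirror is a rotatable laser-puzzle mirror that bounces beams by spawning a new BP_Laser at the hit point.
; The new laser keeps the incoming color, with rotation calculated from the hit normal and beam start.
; Player aim yaws the Arrow from its StartingAngle after a brief delay, destroying the outgoing laser and invalidating the source's hit actor.
; Highlighting toggles the frame's custom depth stencil.
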(event `self.ReceiveBeginPlay`
  (`SceneComponent.K2_SetRelativeRotation` (`self.Arrow`) (`KismetMathLibrary.MakeRotator` 0.0 0.0 (`self.StartingAngle`)) false false))

(event `/Game/LazerContent/BPI_Laser.OnLaserHit`
  (params (LaserColor :type "LinearColor Structure") (LaserHitPos :type "Vector Structure") (LaserHitNormal :type "Vector Structure") (LaserStart :type "Vector Structure") (LaserSrc :type "/Game/LazerContent/BP_Laser Object Reference"))
  (set `self.LaserSource` LaserSrc)
  (bind _returnvalue (`|SpawnActorFromClass` "/Game/LazerContent/BP_Laser.BP_Laser_C" (`KismetMathLibrary.MakeTransform` (+ LaserHitPos LaserHitNormal) (`KismetMathLibrary.MakeRotFromZ` (`KismetMathLibrary.MirrorVectorByNormal` (- LaserHitPos LaserStart) LaserHitNormal))) "Undefined" "MultiplyWithRoot" null LaserColor false null))
  (set `self.Laser` _returnvalue))

(event `/Game/LazerContent/BPI_Laser.OnLaserHitStop`
  (params (LaserID :type "/Game/LazerContent/BP_Laser Object Reference") (LaserColor :type "LinearColor Structure"))
  (`self.K2_DestroyActor` (`self.Laser`)))

(event `/Game/LazerContent/BPI_PlayerInteraction.HighlightStart`
  (`PrimitiveComponent.SetCustomDepthStencilValue` (`self.Mirror_MirrorFrame`) 2))

(event `/Game/LazerContent/BPI_PlayerInteraction.HighlightStop`
  (`PrimitiveComponent.SetCustomDepthStencilValue` (`self.Mirror_MirrorFrame`) 0))

(event `/Game/LazerContent/BPI_PlayerInteraction.InteractAction`
  (params (Interacting :type Boolean) (PlayerAimMovement :type "Vector2D Structure") (PlayerRef :type "/Game/FirstPerson/Blueprints/BP_FirstPersonCharacter Object Reference"))
  (bind _lasersource (`self.LaserSource`))
  (`KismetSystemLibrary.Delay` 0.1)
  (`SceneComponent.K2_AddRelativeRotation` (`self.Arrow`) (`KismetMathLibrary.MakeRotator` 0.0 0.0 (* PlayerAimMovement_X 5.0)) false false)
  (if (`KismetSystemLibrary.IsValid` (`self.Laser`))
    (`self.K2_DestroyActor` (`self.Laser`))
    (if (`KismetSystemLibrary.IsValid` _lasersource)
      (`/Game/LazerContent/BP_Laser.InvalidateHitActor` _lasersource))))

(fn `StartInteract`
  (returns (PlayerIsLocked :type Boolean))
  (return true))

(fn `StopInteract`
  (returns (PlayerIsLocked :type Boolean))
  (return false))

(fn `UserConstructionScript`
  (`SceneComponent.K2_SetRelativeRotation` (`self.Arrow`) (`KismetMathLibrary.MakeRotator` 0.0 0.0 (`self.StartingAngle`)) false false))