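; BP_LaserSensor is a laser puzzle receiver that powers a linked object while a laser of the matching color hits it.
; Construction and BeginPlay each create a dynamic emitter material on the sensor pad tinted to TargetColor, so the color also previews in the editor.
; OnLaserHit and OnLaserHitStop compare the laser's color to TargetColor, toggle the pad's glow intensity and send power enable or disable messages to PowerObject.
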(event `self.ReceiveBeginPlay`
  (bind _returnvalue (`PrimitiveComponent.CreateDynamicMaterialInstance` (`self.LaserSensor_SensorPad`) 0 "/Game/Materials/M_Emitter.M_Emitter" "None"))
  (bind _output_get (set `self.Material` _returnvalue))
  (`MaterialInstanceDynamic.SetVectorParameterValue` _output_get "Color" (`self.TargetColor`)))

(event `/Game/LazerContent/BPI_Laser.OnLaserHit`
  (params (LaserColor :type "LinearColor Structure") (LaserHitPos :type "Vector Structure") (LaserHitNormal :type "Vector Structure") (LaserStart :type "Vector Structure") (LaserSrc :type "/Game/LazerContent/BP_Laser Object Reference"))
  (bind _powerobject (`self.PowerObject`))
  (if (== LaserColor (`self.TargetColor`))
    (`MaterialInstanceDynamic.SetScalarParameterValue` (`self.Material`) "Intensity" 100.0)
    (if (`KismetSystemLibrary.IsValid` _powerobject)
      (message `/Game/LazerContent/BPI_Trigger.OnPowerEnable` _powerobject))))

(event `/Game/LazerContent/BPI_Laser.OnLaserHitStop`
  (params (LaserID :type "/Game/LazerContent/BP_Laser Object Reference") (LaserColor :type "LinearColor Structure"))
  (bind _powerobject (`self.PowerObject`))
  (if (== LaserColor (`self.TargetColor`))
    (`MaterialInstanceDynamic.SetScalarParameterValue` (`self.Material`) "Intensity" 0.0)
    (if (`KismetSystemLibrary.IsValid` _powerobject)
      (message `/Game/LazerContent/BPI_Trigger.OnPowerDisable` _powerobject))))

(fn `UserConstructionScript`
  (bind _returnvalue (`PrimitiveComponent.CreateDynamicMaterialInstance` (`self.LaserSensor_SensorPad`) 0 "/Game/Materials/M_Emitter.M_Emitter" "None"))
  (`MaterialInstanceDynamic.SetVectorParameterValue` _returnvalue "Color" (`self.TargetColor`)))